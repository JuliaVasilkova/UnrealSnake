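; Spawner actor that drops a new food actor into the snake game about once per second, using a Delay on Tick.
; Before each spawn, UpdateSpawnTransform increments an Id, which is passed to the food, and reads the player's BP_SnakePawn.
; Score parity picks which axis mirrors the pawn's negated position, while the other is random within a fixed range at constant height.
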(event EventTick
  (params (DeltaSeconds :type Float%20%28single-precision%29))
  (Utilities|FlowControl|Delay 1.0)
  (CallFunction|UpdateSpawnTransform)
  ;[1 1 1] Spawn of Food actors
  (Game|SpawnActorfromClass "/Game/Blueprints/BP_FoordActor.BP_FoordActor_C" (Variables|Default|GetSpawnTransform) "AdjustIfPossibleButAlwaysSpawn" 0 (Variables|Default|GetId) 0))

(fn ConstructionScript)

(fn UpdateSpawnTransform
  ;[1 1 1] Setup random location to locate spawned actor in scene
  (Math|Integer|IncrementInt (Variables|Default|GetId)
    (:%20%20
      (bind _asbp_snake_pawn (Utilities|Casting|CastToBP_SnakePawn (Game|Player|GetPlayerPawn 0)))
      (LocalVariables|SetPlayerPawn _asbp_snake_pawn)
      (if (Math|Conversions|ToBoolean(Integer) (Math|Integer|%(Integer) (Variables|/Game/Blueprints/BP_SnakePawn.BP_SnakePawn_C|GetScores (LocalVariables|GetPlayerPawn)) 2))
        (bind _output_get (Variables|Default|SetSpawnLocation (Math|Vector|MakeVector (* (.x (Transformation|GetActorLocation (LocalVariables|GetPlayerPawn))) -1.0) (Math|Conversions|ToFloat(Integer) (Math|Random|RandomIntegerinRange -4000 4000)) 2e+01)))
        (Variables|Default|SetSpawnTransform (Math|Conversions|ToTransform(Vector) _output_get))
        (else
          (bind _output_get_2 (Variables|Default|SetSpawnLocation (Math|Vector|MakeVector (Math|Conversions|ToFloat(Integer) (Math|Random|RandomIntegerinRange -4000 4000)) (* (.y (Transformation|GetActorLocation (LocalVariables|GetPlayerPawn))) -1.0) 2e+01)))
          (Variables|Default|SetSpawnTransform (Math|Conversions|ToTransform(Vector) _output_get_2)))))))